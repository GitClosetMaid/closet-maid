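; Global_Functions holds MeasureSpline, a work-in-progress helper that labels spline segment lengths with a text render component when ToggleMeasurements is on.
; It loops over spline points, takes the distance between neighbors, and positions the text at half that length from the spline start, plus a vertical offset.
; Text size scales with segment length, and UnitType selects uu, meters or feet.
; The text reference is cleared after placement, before its rotation, size and text calls.
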(fn `MeasureSpline`
  (params (Spline :type "SplineComponent Object Reference") (TextRender :type "TextRenderComponent Object Reference"))
  (locals (ToggleMeasurements :type Boolean :default true) (NumOfSplinePoints :type Integer) (CurrentPointIndex :type Integer) (SegmentLengthUU :type "Float (double-precision)") (TextVerticalOffset :type "Float (double-precision)" :default 5.0) (DefaultSizeMultiplier :type "Float (double-precision)" :default 0.05) (UnitType :type "/Game/Blueprints/WIP/David_E/SplineTest/UnitTypes Enum" :default "NewEnumerator0") (TextRef :type "TextRenderComponent Object Reference"))
  (bind _currentpointindex (`local.CurrentPointIndex`))
  (bind _returnvalue (- (`SplineComponent.GetDistanceAlongSplineAtSplinePoint` Spline _currentpointindex) (`SplineComponent.GetDistanceAlongSplineAtSplinePoint` Spline (- _currentpointindex 1))))
  (bind (_returnvalue_x _returnvalue_y _returnvalue_z) (`KismetMathLibrary.BreakVector` (`SplineComponent.GetLocationAtDistanceAlongSpline` Spline (+ (/ _returnvalue 2.0) 1.0) "Local")))
  (set `local.TextRef` TextRender)
  (if (`local.ToggleMeasurements`)
    (bind _output_get (set `local.NumOfSplinePoints` (`SplineComponent.GetNumberOfSplinePoints` Spline)))
    (for _index (range (+ _output_get 1))
      (set `local.CurrentPointIndex` _index)
      (if (!= (`local.CurrentPointIndex`) (`local.NumOfSplinePoints`))
        (set `local.SegmentLengthUU` _returnvalue)
        (`SceneComponent.K2_SetRelativeTransform` (`local.TextRef`) (`KismetMathLibrary.MakeTransform` (`KismetMathLibrary.MakeVector` _returnvalue_x _returnvalue_y (+ _returnvalue_z (`local.TextVerticalOffset`))) (struct)) false false)
        (bind _output_get_2 (set `local.TextRef` null))
        (`SceneComponent.SetAbsolute` _output_get_2 false true false)
        (`TextRenderComponent.SetWorldSize` (`local.TextRef`) (* (`local.SegmentLengthUU`) (`local.DefaultSizeMultiplier`)))
        (if (`|EnumEquality` "NewEnumerator0" (`local.UnitType`))
          (`TextRenderComponent.K2_SetText` (`local.TextRef`) (`KismetTextLibrary.Conv_StringToText` (`KismetStringLibrary.Concat_StrStr` (`KismetTextLibrary.Conv_TextToString` (`KismetTextLibrary.Conv_DoubleToText` (`local.SegmentLengthUU`) "HalfToEven" false true 1 324 2 2)) "uu")))
          (elif (`|EnumEquality` "NewEnumerator1" (`local.UnitType`))
            (`TextRenderComponent.K2_SetText` (`local.TextRef`) (`KismetTextLibrary.Conv_StringToText` (`KismetStringLibrary.Concat_StrStr` (`KismetTextLibrary.Conv_TextToString` (`KismetTextLibrary.Conv_DoubleToText` (/ (`local.SegmentLengthUU`) 100.0) "HalfToEven" false true 1 324 2 2)) "m")))
            (elif (`|EnumEquality` "NewEnumerator2" (`local.UnitType`))
              (`TextRenderComponent.K2_SetText` (`local.TextRef`) (`KismetTextLibrary.Conv_StringToText` (`KismetStringLibrary.Concat_StrStr` (`KismetTextLibrary.Conv_TextToString` (`KismetTextLibrary.Conv_DoubleToText` (* (* (/ (`local.SegmentLengthUU`) 100.0) 1.0936) 3.0) "HalfToEven" false true 1 324 2 2)) "ft"))))))))))